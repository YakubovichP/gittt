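; Procedural level tile for the flying game that fills itself with randomly placed traps ("lovushka") and a coin ("monetka").
; The construction script builds rotated spawn transforms from marker components, then adds child actors with FlipFlop-alternated placement and randomized transforms, plus a coin offset from BLOCK5.
; When Maincharacter overlaps the box, it asks FlyingGameMode for another tile and destroys itself after a delay.
; Getattachtransform exposes the AttachPoint world transform.
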(event OnComponentBeginOverlap(Box)
  (params (OverlappedComponent :type Primitive%20Component%20Object%20Reference) (OtherActor :type Actor%20Object%20Reference) (OtherComp :type Primitive%20Component%20Object%20Reference) (OtherBodyIndex :type Integer) (bFromSweep :type Boolean) (SweepResult :type Hit%20Result%20Structure%20%28by%20ref%29))
  (Utilities|Casting|CastToMaincharacter OtherActor)
  (bind _asflying_game_mode (Utilities|Casting|CastToFlyingGameMode (Game|GetGameMode)))
  (Default|Addfloortile _asflying_game_mode false)
  (Utilities|FlowControl|Delay 1.0)
  (Actor|DestroyActor))

(event EventBeginPlay)

(event Collision|EventActorBeginOverlap
  (params (OtherActor :type Actor%20Object%20Reference)))

(event EventTick
  (params (DeltaSeconds :type Float%20%28single-precision%29)))

(fn ConstructionScript
  (CallFunction|SetSpawnpoint)
  (CallFunction|Spawnlovushka)
  (CallFunction|Spawnlovushka)
  (CallFunction|Spawnmonetka))

(fn Getattachtransform
  (return (Transformation|GetWorldTransform (Variables|Components|GetAttachPoint))))

(fn SetSpawnpoint
  (bind _spawnpointr_mid (Variables|Components|Getspawnpointr_MID))
  (bind _spawnpointl_hi (Variables|Components|GetSpawnpointL_HI))
  (bind _spawnpointl_low (Variables|Components|GetspawnpointL_LOW))
  (bind _spawnpointlmid (Variables|Components|GetspawnpointLMID))
  (bind _spawnpointr_hi (Variables|Components|GetSpawnpointr_HI))
  (bind _returnvalue (Transformation|GetRelativeTransform _spawnpointlmid))
  (bind _returnvalue_2 (Transformation|GetRelativeTransform _spawnpointr_hi))
  (bind _returnvalue_3 (Transformation|GetRelativeTransform _spawnpointr_mid))
  (bind _returnvalue_4 (Transformation|GetRelativeTransform _spawnpointl_hi))
  (bind _returnvalue_5 (Transformation|GetRelativeTransform _spawnpointl_low))
  (bind (_roll _pitch _yaw) (Math|Rotator|BreakRotator (.rotation _returnvalue)))
  (bind (_roll_2 _pitch_2 _yaw_2) (Math|Rotator|BreakRotator (.rotation _returnvalue_2)))
  (bind (_roll_3 _pitch_3 _yaw_3) (Math|Rotator|BreakRotator (.rotation _returnvalue_3)))
  (bind (_roll_4 _pitch_4 _yaw_4) (Math|Rotator|BreakRotator (.rotation _returnvalue_4)))
  (bind (_roll_5 _pitch_5 _yaw_5) (Math|Rotator|BreakRotator (.rotation _returnvalue_5)))
  (Variables|Default|Setspawnpoints (Utilities|Array|MakeArray (Math|Transform|MakeTransform (.location _returnvalue_2) (Math|Rotator|MakeRotator _roll_2 (- _pitch_2 9e+01) _yaw_2) (.scale _returnvalue_2)) (Math|Transform|MakeTransform (.location _returnvalue_3) (Math|Rotator|MakeRotator _roll_3 (- _pitch_3 9e+01) _yaw_3) (.scale _returnvalue_3)) (Math|Transform|MakeTransform (.location _returnvalue_4) (Math|Rotator|MakeRotator _roll_4 (+ _pitch_4 2.7e+02) _yaw_4) (.scale _returnvalue_4)) (Math|Transform|MakeTransform (.location _returnvalue_5) (Math|Rotator|MakeRotator _roll_5 (+ _pitch_5 2.7e+02) _yaw_5) (.scale _returnvalue_5)) (Math|Transform|MakeTransform (.location _returnvalue) (Math|Rotator|MakeRotator _roll (+ _pitch 2.7e+02) _yaw) (.scale _returnvalue)))))

(fn Spawnlovushka
  (bind _returnvalue (Math|Random|RandomFloatinRange 1.0 1.1))
  (bind _spawnpoints (Variables|Default|Getspawnpoints))
  (bind _returnvalue_2 (Utilities|Array|LastIndex _spawnpoints))
  (bind _returnvalue_3 (Math|Random|RandomIntegerinRange 0 _returnvalue_2))
  (bind _output (Utilities|Array|Get(acopy) _spawnpoints _returnvalue_3))
  (bind (_x _y _z) (Math|Vector|BreakVector (.location _output)))
  (for _index (range 0 3)
    (Utilities|FlowControl|FlipFlop
      (:A
        (AddComponent|AddChildActorComponent false (Math|Transform|MakeTransform (Math|Vector|MakeVector _x (Math|Random|RandomFloatinRange _y (+ _y 2e+02)) (Math|Random|RandomFloatinRange _z (+ _z 2e+02))) (.rotation _output) (Math|Vector|MakeVector 1.0 1.0 _returnvalue))))
      (:B
        (AddComponent|AddChildActorComponent false (Math|Transform|MakeTransform (.location _output) (.rotation _output) (Math|Vector|MakeVector _returnvalue _returnvalue _returnvalue)))))))

(fn Spawnmonetka
  (bind _block_5 (Variables|Default|GetBLOCK_5))
  (bind _returnvalue (Transformation|GetRelativeTransform _block_5))
  (bind (_location _rotation) (Math|Transform|BreakTransform _returnvalue))
  (AddComponent|AddChildActorComponent false (Math|Transform|MakeTransform (+ _location (Math|Vector|MakeVector (Math|Random|RandomFloatinRange 5e+01 2e+02) (Math|Random|RandomFloatinRange 5e+01 2e+02) (Math|Random|RandomFloatinRange 5e+01 2e+02))) _rotation)))