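; Blade trap hazard that swings endlessly and kills the main character on contact.
; Two timelines lerp the blade mesh's relative rotation to slam it down and raise it, chaining through the Slam event in a loop that BeginPlay starts with the raise.
; A hit on the Maincharacter calls its Death function once, then reloads the current level after a short delay.
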(event Custom|Slam
  ;[1 1 1] Slam the player
  (bind _newtrack_0 (Timeline|Timeline_0 PlayFromStart) ; Timeline updates blade position
    (:Update
      (Transformation|SetRelativeRotation (Variables|Default|Getm_blade_01) (Math|Rotator|Lerp(Rotator) "0, 0,-90.000000" "0, 0, 0" _newtrack_0) false false) ; Uses vector to set new rotation
    )
    (:Finished
      ;[1 1 1] Raise the blade
      (bind _newtrack_0_2 (Timeline|Timeline_1 PlayFromStart) ; Timeline updates blade position
        (:Update
          (Transformation|SetRelativeRotation (Variables|Default|Getm_blade_01) (Math|Rotator|Lerp(Rotator) "0, 0, 0" "0.000000, 0,-90.000000" _newtrack_0_2) false false) ; Uses vector to set new rotation
        )
        (:Finished
          (CallFunction|Slam) ; Blade is up - slam the player
        )))))

(event Collision|EventHit
  (params (MyComp :type Primitive%20Component%20Object%20Reference) (Other :type Actor%20Object%20Reference) (OtherComp :type Primitive%20Component%20Object%20Reference) (bSelfMoved :type Boolean) (HitLocation :type Vector :default "0, 0, 0") (HitNormal :type Vector :default "0, 0, 0") (NormalImpulse :type Vector :default "0, 0, 0") (Hit :type Hit%20Result%20Structure%20%28by%20ref%29))
  (bind _asmaincharacter (Utilities|Casting|CastToMaincharacter Other))
  (Utilities|FlowControl|DoOnce false
    (:Completed
      (Default|Death _asmaincharacter)
      (Utilities|FlowControl|Delay 2.0)
      (bind _returnvalue (Game|GetCurrentLevelName true))
      (Game|OpenLevel(byName) (Utilities|String|StringToName _returnvalue)))))

(event EventBeginPlay
  ;[1 1 1] Raise the blade
  (bind _newtrack_0 (Timeline|Timeline_1 Play) ; Timeline updates blade position
    (:Update
      (Transformation|SetRelativeRotation (Variables|Default|Getm_blade_01) (Math|Rotator|Lerp(Rotator) "0, 0, 0" "0.000000, 0,-90.000000" _newtrack_0) false false) ; Uses vector to set new rotation
    )
    (:Finished
      (CallFunction|Slam) ; Blade is up - slam the player
    )))

(fn ConstructionScript)