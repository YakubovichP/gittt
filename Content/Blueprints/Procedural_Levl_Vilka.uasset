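; Forked level tile actor for procedural floor generation in a flying game, exposing two attach points.
; When the main character overlaps the right spawn box, it calls Addfloortile1 on FlyingGameMode with false, then destroys itself after one second.
; Getattachtransform returns both attach points' world transforms, with the left output taken from AttachPointRight and the right from AttachPointLeft.
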(event OnComponentBeginOverlap(rightspawnbox)
  (params (OverlappedComponent :type Primitive%20Component%20Object%20Reference) (OtherActor :type Actor%20Object%20Reference) (OtherComp :type Primitive%20Component%20Object%20Reference) (OtherBodyIndex :type Integer) (bFromSweep :type Boolean) (SweepResult :type Hit%20Result%20Structure%20%28by%20ref%29))
  (Utilities|Casting|CastToMaincharacter OtherActor)
  (bind _asflying_game_mode (Utilities|Casting|CastToFlyingGameMode (Game|GetGameMode)))
  (Default|Addfloortile1 _asflying_game_mode false)
  (Utilities|FlowControl|Delay 1.0)
  (Actor|DestroyActor))

(event EventBeginPlay)

(event Collision|EventActorBeginOverlap
  (params (OtherActor :type Actor%20Object%20Reference)))

(event EventTick
  (params (DeltaSeconds :type Float%20%28single-precision%29)))

(fn ConstructionScript)

(fn Getattachtransform
  (return (Transformation|GetWorldTransform (Variables|Components|GetAttachPoint_right)) (Transformation|GetWorldTransform (Variables|Default|GetAttachPoint_left))))