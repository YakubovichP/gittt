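; Procedural level tile for the flying game: when Maincharacter overlaps its box, it calls Addfloortile1 on FlyingGameMode, then destroys itself a second later.
; Getattachtransform exposes the AttachPoint world transform.
; Construction builds three rotated spawn transforms from marker components and adds a child actor (a coin, "monetka", by name) at a random offset from BLOCK1.
; Spawnlovushka (trap) is called twice but does nothing, as its random-placement logic is disconnected.
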(event OnComponentBeginOverlap(Box)
  (params (OverlappedComponent :type Primitive%20Component%20Object%20Reference) (OtherActor :type Actor%20Object%20Reference) (OtherComp :type Primitive%20Component%20Object%20Reference) (OtherBodyIndex :type Integer) (bFromSweep :type Boolean) (SweepResult :type Hit%20Result%20Structure%20%28by%20ref%29))
  (Utilities|Casting|CastToMaincharacter OtherActor)
  (bind _asflying_game_mode (Utilities|Casting|CastToFlyingGameMode (Game|GetGameMode)))
  (Default|Addfloortile1 _asflying_game_mode false)
  (Utilities|FlowControl|Delay 1.0)
  (Actor|DestroyActor))

(event EventBeginPlay)

(event Collision|EventActorBeginOverlap
  (params (OtherActor :type Actor%20Object%20Reference)))

(event EventTick
  (params (DeltaSeconds :type Float%20%28single-precision%29)))

(fn ConstructionScript
  (CallFunction|SetSpawnpoint)
  (CallFunction|Spawnlovushka)
  (CallFunction|Spawnlovushka)
  (CallFunction|Spawnmonetka))

(fn Getattachtransform
  (return (Transformation|GetWorldTransform (Variables|Components|GetAttachPoint))))

(fn SetSpawnpoint
  (bind _spawnpointr_low (Variables|Components|GetSpawnpointr_LOW))
  (bind _spawnpointr_mid (Variables|Components|Getspawnpointr_MID))
  (bind _spawnpointl_low (Variables|Components|GetspawnpointL_LOW))
  (bind _returnvalue (Transformation|GetRelativeTransform _spawnpointr_low))
  (bind _returnvalue_2 (Transformation|GetRelativeTransform _spawnpointr_mid))
  (bind _returnvalue_3 (Transformation|GetRelativeTransform _spawnpointl_low))
  (bind (_roll _pitch _yaw) (Math|Rotator|BreakRotator (.rotation _returnvalue)))
  (bind (_roll_2 _pitch_2 _yaw_2) (Math|Rotator|BreakRotator (.rotation _returnvalue_2)))
  (bind (_roll_3 _pitch_3 _yaw_3) (Math|Rotator|BreakRotator (.rotation _returnvalue_3)))
  (Variables|Default|Setspawnpoints (Utilities|Array|MakeArray (Math|Transform|MakeTransform (.location _returnvalue) (Math|Rotator|MakeRotator _roll (- _pitch 9e+01) _yaw) (.scale _returnvalue)) (Math|Transform|MakeTransform (.location _returnvalue_2) (Math|Rotator|MakeRotator _roll_2 (- _pitch_2 9e+01) _yaw_2) (.scale _returnvalue_2)) (Math|Transform|MakeTransform (.location _returnvalue_3) (Math|Rotator|MakeRotator _roll_3 (+ _pitch_3 2.7e+02) _yaw_3) (.scale _returnvalue_3)))))

(fn Spawnlovushka)

(fn Spawnmonetka
  (bind _block_1 (Variables|Default|GetBLOCK_1))
  (bind _returnvalue (Transformation|GetRelativeTransform _block_1))
  (bind (_location _rotation) (Math|Transform|BreakTransform _returnvalue))
  (AddComponent|AddChildActorComponent false (Math|Transform|MakeTransform (+ _location (Math|Vector|MakeVector (Math|Random|RandomFloatinRange 5e+01 2e+02) (Math|Random|RandomFloatinRange 5e+01 2e+02) (Math|Random|RandomFloatinRange 5e+01 2e+02))) _rotation)))