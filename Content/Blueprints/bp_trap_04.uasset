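; Mace trap Blueprint that swings a mace when something overlaps its trigger, as a one-shot hazard meant to slam the player.
; A timeline lerps the mace's relative rotation down through its arc, then calls Reset, whose second timeline swings it back.
; DoOnce is set only after the return swing finishes, blocking later triggers.
; The overlap has no actor filter, and the graph applies no damage or force.
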(event OnComponentBeginOverlap(trigger_01)
  (params (OverlappedComponent :type Primitive%20Component%20Object%20Reference) (OtherActor :type Actor%20Object%20Reference) (OtherComp :type Primitive%20Component%20Object%20Reference) (OtherBodyIndex :type Integer) (bFromSweep :type Boolean) (SweepResult :type Hit%20Result%20Structure%20%28by%20ref%29))
  ;[1 1 1] Slam the player
  (if (not (Variables|Default|GetDoOnce)) ; If DoOnce is 0
    (bind _newtrack_0 (Timeline|Timeline_0 Play) ; Timeline updates mace position
      (:Update
        (Transformation|SetRelativeRotation (Variables|Default|Getm_macetrap_02) (Math|Rotator|Lerp(Rotator) "0.000000,0.000000,170.000000" "0.000000, 0,70.000000" _newtrack_0) false false) ; Uses vector to set new rotation
      )
      (:Finished
        (CallFunction|Reset) ; Reset the trap
      ))))

(event Custom|Reset
  ;[1 1 1] Reset
  (bind _newtrack_0 (Timeline|Timeline_1 PlayFromStart) ; Timeline updates mace position
    (:Update
      (Transformation|SetRelativeRotation (Variables|Default|Getm_macetrap_02) (Math|Rotator|Lerp(Rotator) "0.000000,0.000000,70.000000" "0.000000, 0,170.000000" _newtrack_0) false false) ; Uses vector to set new rotation
    )
    (:Finished
      (Variables|Default|SetDoOnce true) ; Set DoOnce to 1
    )))

(fn ConstructionScript)