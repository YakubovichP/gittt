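; Circular saw hazard actor that kills the main character on contact.
; Tick keeps calling Play on a timeline that lerps the main static mesh's relative yaw through a full turn to spin it.
; Hit events on five static mesh components each cast the other actor to Maincharacter and call Death.
; A second timeline for shifting the actor along X is left unconnected and never runs.
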(event OnComponentHit(StaticMesh)
  (params (HitComponent :type Primitive%20Component%20Object%20Reference) (OtherActor :type Actor%20Object%20Reference) (OtherComp :type Primitive%20Component%20Object%20Reference) (NormalImpulse :type Vector :default "0, 0, 0") (Hit :type Hit%20Result%20Structure%20%28by%20ref%29))
  (bind _asmaincharacter (Utilities|Casting|CastToMaincharacter OtherActor))
  (Default|Death _asmaincharacter))

(event OnComponentHit(StaticMesh1)
  (params (HitComponent :type Primitive%20Component%20Object%20Reference) (OtherActor :type Actor%20Object%20Reference) (OtherComp :type Primitive%20Component%20Object%20Reference) (NormalImpulse :type Vector :default "0, 0, 0") (Hit :type Hit%20Result%20Structure%20%28by%20ref%29))
  (bind _asmaincharacter (Utilities|Casting|CastToMaincharacter OtherActor))
  (Default|Death _asmaincharacter))

(event OnComponentHit(StaticMesh2)
  (params (HitComponent :type Primitive%20Component%20Object%20Reference) (OtherActor :type Actor%20Object%20Reference) (OtherComp :type Primitive%20Component%20Object%20Reference) (NormalImpulse :type Vector :default "0, 0, 0") (Hit :type Hit%20Result%20Structure%20%28by%20ref%29))
  (bind _asmaincharacter (Utilities|Casting|CastToMaincharacter OtherActor))
  (Default|Death _asmaincharacter))

(event OnComponentHit(StaticMesh3)
  (params (HitComponent :type Primitive%20Component%20Object%20Reference) (OtherActor :type Actor%20Object%20Reference) (OtherComp :type Primitive%20Component%20Object%20Reference) (NormalImpulse :type Vector :default "0, 0, 0") (Hit :type Hit%20Result%20Structure%20%28by%20ref%29))
  (bind _asmaincharacter (Utilities|Casting|CastToMaincharacter OtherActor))
  (Default|Death _asmaincharacter))

(event OnComponentHit(StaticMesh4)
  (params (HitComponent :type Primitive%20Component%20Object%20Reference) (OtherActor :type Actor%20Object%20Reference) (OtherComp :type Primitive%20Component%20Object%20Reference) (NormalImpulse :type Vector :default "0, 0, 0") (Hit :type Hit%20Result%20Structure%20%28by%20ref%29))
  (bind _asmaincharacter (Utilities|Casting|CastToMaincharacter OtherActor))
  (Default|Death _asmaincharacter))

(event EventBeginPlay)

(event Collision|EventActorBeginOverlap
  (params (OtherActor :type Actor%20Object%20Reference)))

(event EventTick
  (params (DeltaSeconds :type Float%20%28single-precision%29))
  (bind _newtrack_0 (Timeline|Timeline_0 Play)
    (:Update
      (Transformation|SetRelativeRotation (Variables|Default|GetStaticMesh) (Math|Rotator|MakeRotator 0.0 0.0 (Math|Float|Lerp 3.6e+02 0.0 _newtrack_0)) false false))))

(fn ConstructionScript)