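; Circular saw hazard that kills the Maincharacter on hit and reloads the current level after a short delay.
; At BeginPlay, if the player is alive, a timeline moves the mesh along a relative X/Y/Z diagonal.
; A Sphere overlap briefly lowers global time dilation for slow motion, leaving the player's custom dilation at normal.
; A DoOnce limits the death sequence to one run.
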(event OnComponentBeginOverlap(Sphere)
  (params (OverlappedComponent :type Primitive%20Component%20Object%20Reference) (OtherActor :type Actor%20Object%20Reference) (OtherComp :type Primitive%20Component%20Object%20Reference) (OtherBodyIndex :type Integer) (bFromSweep :type Boolean) (SweepResult :type Hit%20Result%20Structure%20%28by%20ref%29))
  (bind _asmaincharacter (Utilities|Casting|CastToMaincharacter OtherActor))
  (Utilities|Time|SetGlobalTimeDilation 0.2)
  (Variables|/Script/Engine.Actor|SetCustomTimeDilation _asmaincharacter 1.0)
  (Utilities|FlowControl|Delay 0.2)
  (Utilities|Time|SetGlobalTimeDilation 1.0)
  (Variables|/Script/Engine.Actor|SetCustomTimeDilation _asmaincharacter 1.0))

(event EventBeginPlay
  (bind _asmaincharacter (Utilities|Casting|CastToMaincharacter (Game|Player|GetPlayerPawn 0)))
  (Variables|Default|Setpawn _asmaincharacter)
  (if (Variables|/Game/FlyingBP/Blueprints/Maincharacter.Maincharacter_C|Getisalive? (Variables|Default|Getpawn))
    (bind _newtrack_0 (Timeline|Timeline_0 Play)
      (:Update
        (Transformation|SetRelativeLocation (Variables|Default|GetStaticMesh) (Math|Vector|MakeVector (Math|Float|Lerp -2e+01 2e+01 _newtrack_0) (Math|Float|Lerp -2e+01 2e+01 _newtrack_0) (Math|Float|Lerp -2e+01 2e+01 _newtrack_0)) false false)))
    (else
      (Timeline|Timeline_0 Stop))))

(event Collision|EventHit
  (params (MyComp :type Primitive%20Component%20Object%20Reference) (Other :type Actor%20Object%20Reference) (OtherComp :type Primitive%20Component%20Object%20Reference) (bSelfMoved :type Boolean) (HitLocation :type Vector :default "0, 0, 0") (HitNormal :type Vector :default "0, 0, 0") (NormalImpulse :type Vector :default "0, 0, 0") (Hit :type Hit%20Result%20Structure%20%28by%20ref%29))
  (bind _asmaincharacter (Utilities|Casting|CastToMaincharacter Other))
  (Utilities|FlowControl|DoOnce false
    (:Completed
      (Default|Death _asmaincharacter)
      (Utilities|FlowControl|Delay 2.0)
      (bind _returnvalue (Game|GetCurrentLevelName true))
      (Game|OpenLevel(byName) (Utilities|String|StringToName _returnvalue)))))

(fn ConstructionScript)